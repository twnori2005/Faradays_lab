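; Configurable alembic prop that sets up its look entirely in the Construction Script, with no active runtime logic.
; Exposed variables drive dynamic material instances for glass tint, liquid color, opacity and bubbling, and a drip that takes the liquid's top color.
; Toggles show the liquid, tag and drip, and the tag's sign-flip parameter is randomized on each construction.
; Brass or Copper choices replace the glass material and hide the liquid.
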(fn `UserConstructionScript`
  (bind _liquid (`self.liquid`))
  (bind _sm_tag_002 (`self.SM_Tag_002`))
  (bind _p_drip_001 (`self.P_Drip_001`))
  (if (`self.Add Liquid`)
    (`SceneComponent.SetVisibility` _liquid true false)
    (else
      (`SceneComponent.SetVisibility` _liquid false false)))
  (`PrimitiveComponent.SetTranslucentSortPriority` (`self.test`) 1)
  (bind _returnvalue (`PrimitiveComponent.CreateDynamicMaterialInstance` (`self.liquid`) 0 "/Game/Materials/MeshMats/MI_Glassware_Liquid_001.MI_Glassware_Liquid_001"))
  (`MaterialInstanceDynamic.SetScalarParameterValue` _returnvalue "Bubbling_Intensity" (`self.Liquid Bubbling Amount`))
  (`MaterialInstanceDynamic.SetScalarParameterValue` _returnvalue "Bubbling_MAX" (`self.Bubbling MAX`))
  (`MaterialInstanceDynamic.SetScalarParameterValue` _returnvalue "Bubbling_MIN" (`self.Bubbling MIN`))
  (`MaterialInstanceDynamic.SetVectorParameterValue` _returnvalue "Color_Top" (`self.Liquid Color Top`))
  (`MaterialInstanceDynamic.SetVectorParameterValue` _returnvalue "Color_Bottom" (`self.Liquid Color Bottom`))
  (`MaterialInstanceDynamic.SetScalarParameterValue` _returnvalue "Opacity Top" (`self.Liquid Opacity Top`))
  (`MaterialInstanceDynamic.SetScalarParameterValue` _returnvalue "Opacity Bottom" (`self.Liquid Opacity Bottom`))
  (bind _returnvalue_2 (`PrimitiveComponent.CreateDynamicMaterialInstance` (`self.test`) 0 "/Game/Materials/MeshMats/MI_Glassware_001_Change_This_And_The_Rest_Will_Follow.MI_Glassware_001_Change_This_And_The_Rest_Will_Follow"))
  (`MaterialInstanceDynamic.SetScalarParameterValue` _returnvalue_2 "Hue shift percentage" (`self.Glass Hue Shift`))
  (`MaterialInstanceDynamic.SetVectorParameterValue` _returnvalue_2 "Color Multiplier" (`self.Glass Color Multiplier`))
  (bind _returnvalue_3 (`PrimitiveComponent.CreateDynamicMaterialInstance` _sm_tag_002 0 "/Game/Materials/MeshMats/MI_Tags_001.MI_Tags_001"))
  (`MaterialInstanceDynamic.SetScalarParameterValue` _returnvalue_3 "Flip between signs" (`KismetMathLibrary.RandomFloatInRange` 0.0 1.0))
  (`SceneComponent.SetVisibility` _sm_tag_002 (`self.Tag`) false)
  (`SceneComponent.SetVisibility` _p_drip_001 (`self.Drip`) false)
  (bind _returnvalue_4 (`PrimitiveComponent.CreateDynamicMaterialInstance` _p_drip_001 0 "/Game/Materials/MeshMats/MI_Drip_001.MI_Drip_001"))
  (`MaterialInstanceDynamic.SetVectorParameterValue` _returnvalue_4 "Color" (`self.Liquid Color Top`))
  (switch `/Game/Materials/MeshMats/ENUM_Alambil_Material_Selection_001` (`self.Choose Alambic Material`)
    (:`NewEnumerator1`
      (`SceneComponent.SetVisibility` (`self.liquid`) false false)
      (`PrimitiveComponent.SetMaterial` (`self.test`) 0 "/Game/Materials/MeshMats/MI_Alambic_Brass_001.MI_Alambic_Brass_001"))
    (:`NewEnumerator2`
      (`SceneComponent.SetVisibility` (`self.liquid`) false false)
      (`PrimitiveComponent.SetMaterial` (`self.test`) 0 "/Game/Materials/MeshMats/MI_Alambic_Copper_001.MI_Alambic_Copper_001"))))