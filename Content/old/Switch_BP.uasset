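; Switch Blueprint that toggles a circuit state when something stops overlapping its static mesh.
; After a short delay, it closes the circuit and turns green, or opens it and turns red if already closed.
; A closed switch also opens itself after AutoOffDuration.
; Each path sets IsCircuitClosed and broadcasts it through SwitchToggled.
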(event `self.StaticMeshComponent.OnComponentEndOverlap`
  (params (OverlappedComponent :type "PrimitiveComponent Object Reference") (OtherActor :type "Actor Object Reference") (OtherComp :type "PrimitiveComponent Object Reference") (OtherBodyIndex :type Integer))
  (bind _staticmeshcomponent (`self.StaticMeshComponent`))
  (`KismetSystemLibrary.Delay` 0.2)
  (if (not (`self.isCircuitClosed`))
    (`PrimitiveComponent.SetMaterial` _staticmeshcomponent 0 "/Game/old/m_green.m_green")
    (bind _output_get (set `self.isCircuitClosed` true))
    (`self.switchToggled` _output_get)
    (`KismetSystemLibrary.Delay` (`self.auto_off_duration`)))
  (`PrimitiveComponent.SetMaterial` _staticmeshcomponent 0 "/Game/old/m_red.m_red")
  (bind _output_get_2 (set `self.isCircuitClosed` false))
  (`self.switchToggled` _output_get_2))

(event `self.StaticMeshComponent.OnComponentBeginOverlap`
  (params (OverlappedComponent :type "PrimitiveComponent Object Reference") (OtherActor :type "Actor Object Reference") (OtherComp :type "PrimitiveComponent Object Reference") (OtherBodyIndex :type Integer) (bFromSweep :type Boolean) (SweepResult :type "HitResult Structure (by ref)")))

(fn `UserConstructionScript`)