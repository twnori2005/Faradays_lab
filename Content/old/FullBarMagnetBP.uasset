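; Bar magnet actor that visualizes magnetism with a Magtron particle component and toggleable magnetic field lines.
; The updateSpawnRate event passes a new rate to Magtron's spawnMagRate float parameter.
; The updateMagFieldViz event flips IsForceLinesOn and applies it to the field lines' visibility, without propagating to children.
; BeginPlay is empty, and a delayed hide of the field lines is left unconnected.
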(event `self.ReceiveBeginPlay`)

(event `updateSpawnRate`
  (params (NewSpawnRate :type "Float (double-precision)"))
  (`self.setSpawnMagRate` NewSpawnRate))

(event `updateMagFieldViz`
  (`self.toggleMagFieldLines`))

(fn `setSpawnMagRate`
  (params (spawnRate :type "Float (double-precision)"))
  (`ParticleSystemComponent.SetFloatParameter` (`self.magtron`) "spawnMagRate" spawnRate))

(fn `toggleMagFieldLines`
  (bind _output_get (set `self.isForceLinesOn` (not (`self.isForceLinesOn`))))
  (`SceneComponent.SetVisibility` (`self.magnetic_field_lines`) _output_get false))

(fn `UserConstructionScript`)